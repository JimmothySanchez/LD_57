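; Player controller for a Ludum Dare 57 game that handles grid-based structure placement with the mouse cursor.
; On BeginPlay it sets up Enhanced Input and the HUD; a screenshot action runs HighResShot.
; Tick snaps the cursor hit to a ground-plane grid, sphere-overlaps for occupancy and shows a red or green debug sphere.
; Select spawns the current build selection on free cells if BrickCount covers its cost, then clears the selection.
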(event Input|EnhancedActionEvents|EnhancedInputActionIA_ScreenShot
  (params (ActionValue :type Boolean) (ElapsedSeconds :type Float%20%28double-precision%29) (TriggeredSeconds :type Float%20%28double-precision%29) (InputAction :type Input%20Action%20Object%20Reference :default "/Game/LD57_Custom/Input/IA_ScreenShot.IA_ScreenShot"))
  (Development|ExecuteConsoleCommand (Utilities|String|ToString(Text) (Utilities|Text|FormatText "HighResShot {mult}" (Utilities|Text|MakeLiteralText "1.5"))) 0))

(event Input|EnhancedActionEvents|EnhancedInputActionIA_Select
  (params (ActionValue :type Boolean) (ElapsedSeconds :type Float%20%28double-precision%29) (TriggeredSeconds :type Float%20%28double-precision%29) (InputAction :type Input%20Action%20Object%20Reference :default "/Game/LD57_Custom/Input/IA_Select.IA_Select"))
  (bind (_hitresult _returnvalue) (Game|Player|GetHitResultUnderCursorbyChannel "TraceTypeQuery1" true))
  (:Completed
    (if _returnvalue
      (bind (_validlocation _isoccupied) (CallFunction|GetNearestValidBuildLocation (.Location (Collision|BreakHitResult _hitresult))))
      (if (not _isoccupied)
        (CallFunction|TryBuildStructure _validlocation)))))

(event EventBeginPlay
  (Input|AddMappingContext (PlayerController|LocalPlayerSubsystems|GetEnhancedInputLocalPlayerSubsystem self) "/Game/LD57_Custom/Input/IMC_Default.IMC_Default" 0 "(bIgnoreAllPressedKeysUntilRelease=True,bForceImmediately=False,bNotifyUserSettings=False)")
  (bind _returnvalue (UserInterface|CreateWidget "/Game/LD57_Custom/Blueprints/UI/WDG_HUD.WDG_HUD_C"))
  (UserInterface|Viewport|AddtoPlayerScreen _returnvalue)
  (Input|SetInputModeGameandUI self _returnvalue "DoNotLock" true false)
  (Variables|Default|SetbShowMouseCursor true))

(event EventTick
  (params (DeltaSeconds :type Float%20%28single-precision%29))
  (bind (_hitresult _returnvalue) (Game|Player|GetHitResultUnderCursorbyChannel "TraceTypeQuery1" true))
  (if _returnvalue
    (bind (_validlocation _isoccupied) (CallFunction|GetNearestValidBuildLocation (.Location (Collision|BreakHitResult _hitresult))))
    (if _isoccupied
      (Rendering|Debug|DrawDebugSphere _validlocation 5e+01 12 "(R=1.000000,G=0.010417,B=0.010417,A=1.000000)" 0.0)
      (else
        (Rendering|Debug|DrawDebugSphere _validlocation 5e+01 12 "(R=0.082564,G=1.000000,B=0.000000,A=1.000000)" 0.0)))))

(fn ConstructionScript)

(fn GetNearestValidBuildLocation
  (params (DesiredLocation :type Vector))
  (bind (_x _y) (Math|Vector|BreakVector DesiredLocation))
  (bind _returnvalue (Math|Float|SnapToGrid(Float) _y 1e+02))
  (bind _returnvalue_2 (Math|Float|SnapToGrid(Float) _x 1e+02))
  (bind _returnvalue_3 (Math|Vector|MakeVector _returnvalue_2 _returnvalue 0.0))
  (bind (_x_2 _y_2 _z) (Math|Vector|BreakVector _returnvalue_3))
  (bind _returnvalue_4 (Collision|SphereOverlapActors (Math|Vector|MakeVector _x_2 _y_2 (+ _z 1e+02)) 5e+01 (Utilities|Array|MakeArray "ObjectTypeQuery2" "ObjectTypeQuery1") 0))
  (return _returnvalue_3 _returnvalue_4))

(fn TryBuildStructure
  (params (BuildLocation :type Vector))
  (Utilities|IsValid (Variables|Default|GetCurrentBuildSelection)
    (:Is%20Valid
      (if (>= (Variables|Default|GetBrickCount) (Variables|/Game/LD57_Custom/DataAssets/PDA_Structure.PDA_Structure_C|GetBrickCost (Variables|Default|GetCurrentBuildSelection)))
        (Game|SpawnActorfromClass (Variables|/Game/LD57_Custom/DataAssets/PDA_Structure.PDA_Structure_C|GetClassType (Variables|Default|GetCurrentBuildSelection)) (Math|Transform|MakeTransform BuildLocation "0, 0, 0" "1.000000,1.000000,1.000000") "Undefined" "MultiplyWithRoot" 0 0)
        (Variables|Default|SetBrickCount (- (Variables|Default|GetBrickCount) (Variables|/Game/LD57_Custom/DataAssets/PDA_Structure.PDA_Structure_C|GetBrickCost (Variables|Default|GetCurrentBuildSelection))))
        (Variables|Default|SetCurrentBuildSelection 0)
        (else
          (Variables|Default|SetCurrentBuildSelection 0))))))