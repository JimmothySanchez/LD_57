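; BP_BrickMaker is a structure that produces bricks for the player over time.
; A looping timer adds bricks to the player controller's count and spawns a Niagara effect each cycle.
; Tick pulses the mesh scale and swings the handle from the game mode's Tempo value.
; Hits on its box by a "wrecking-ball" tagged actor trigger camera shake and a brick burst, then destroy it.
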(event OnComponentHit(StaticMesh)
  (params (HitComponent :type Primitive%20Component%20Object%20Reference) (OtherActor :type Actor%20Object%20Reference) (OtherComp :type Primitive%20Component%20Object%20Reference) (NormalImpulse :type Vector :default "0, 0, 0") (Hit :type Hit%20Result%20Structure%20%28by%20ref%29)))

(event OnComponentHit(Box)
  (params (HitComponent :type Primitive%20Component%20Object%20Reference) (OtherActor :type Actor%20Object%20Reference) (OtherComp :type Primitive%20Component%20Object%20Reference) (NormalImpulse :type Vector :default "0, 0, 0") (Hit :type Hit%20Result%20Structure%20%28by%20ref%29))
  (if (Actor|ActorHasTag OtherActor "wrecking-ball")
    (Utilities|FlowControl|Sequence
      (:then_0
        (Game|Feedback|ClientStartCameraShake (Game|GetPlayerController 0) "/Game/LD57_Custom/Effects/BP_CameraShake.BP_CameraShake_C" 1.0 "World" "0, 0, 0"))
      (:then_1
        (Niagara|SpawnSystematLocation "/Game/LD57_Custom/Effects/NS_BrickBurst.NS_BrickBurst" (Transformation|GetActorLocation)))
      (:then_2
        (Actor|DestroyActor)))))

(event Custom|MakeBricks
  (Variables|/Game/LD57_Custom/Blueprints/Logic/PC_LD57.PC_LD57_C|SetBrickCount (Variables|Default|GetAs%20PC%20LD57) (+ (Variables|/Game/LD57_Custom/Blueprints/Logic/PC_LD57.PC_LD57_C|GetBrickCount (Variables|Default|GetAs%20PC%20LD57)) (Variables|Default|GetBricksPerUpdate)))
  (Niagara|SpawnSystematLocation "/Game/LD57_Custom/Effects/NS_SingleBrick.NS_SingleBrick" (Transformation|GetWorldLocation (Variables|Default|GetScene))))

(event EventBeginPlay
  (Utilities|FlowControl|Sequence
    (:then_0
      (bind _asgm_ld57 (Utilities|Casting|CastToGM_LD57 (Game|GetGameMode)))
      (Variables|Default|SetAs%20GM%20LD57 _asgm_ld57))
    (:then_1
      (bind _aspc_ld57 (Utilities|Casting|CastToPC_LD57 (Game|GetPlayerController 0)))
      (Variables|Default|SetAs%20PC%20LD57 _aspc_ld57))
    (:then_2
      (Utilities|Time|SetTimerbyEvent (delegate Custom|MakeBricks) (Variables|Default|GetBrickCooldown) true))))

(event Collision|EventActorBeginOverlap
  (params (OtherActor :type Actor%20Object%20Reference)))

(event EventTick
  (params (DeltaSeconds :type Float%20%28single-precision%29))
  (bind _as_gm_ld57 (Variables|Default|GetAs%20GM%20LD57))
  (bind _tempo (Variables|/Game/LD57_Custom/Blueprints/Logic/GM_LD57.GM_LD57_C|GetTempo _as_gm_ld57))
  (bind _returnvalue (Math|Float|Lerp 0.95 1.0 _tempo))
  (Transformation|SetRelativeScale3D (Variables|Default|GetStaticMesh) (Math|Vector|MakeVector _returnvalue _returnvalue _returnvalue))
  (Transformation|SetRelativeRotation (Variables|Default|GetBrickMaker_Handle) (Math|Rotator|Lerp(Rotator) "-45.000000,0.000000,0.000000" "45.000000,0.000000,0.000000" _tempo) false false))

(fn ConstructionScript)