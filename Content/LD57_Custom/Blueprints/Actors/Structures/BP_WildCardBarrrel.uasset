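; Breakable barrel structure that shatters when struck by an actor tagged "wrecking-ball".
; The box hit event shakes the first player's camera, destroys the barrel component and adds a GC_Barrel geometry collection in its place as debris.
; BeginPlay caches the LD57 game mode, but the tempo-driven scale pulse that reads it is disconnected, as are the radial impulse and actor destruction.
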(event OnComponentHit(Box)
  (params (HitComponent :type Primitive%20Component%20Object%20Reference) (OtherActor :type Actor%20Object%20Reference) (OtherComp :type Primitive%20Component%20Object%20Reference) (NormalImpulse :type Vector :default "0, 0, 0") (Hit :type Hit%20Result%20Structure%20%28by%20ref%29))
  (if (Actor|ActorHasTag OtherActor "wrecking-ball")
    (Utilities|FlowControl|Sequence
      (:then_0
        (Game|Feedback|ClientStartCameraShake (Game|GetPlayerController 0) "/Game/LD57_Custom/Effects/BP_CameraShake.BP_CameraShake_C" 1.0 "World" "0, 0, 0"))
      (:then_1
        (Components|DestroyComponent (Variables|Default|GetBarrel)))
      (:then_2
        (bind _returnvalue (AddComponent|AddGeometryCollectionComponent false))
        (Class|GeometryCollectionComponent|SetRestCollection _returnvalue "/Game/LD57_Custom/StaticMeshes/Fractures/GC_Barrel.GC_Barrel" true)
        (Transformation|SetRelativeLocation _returnvalue "0.000000,0.000000,-50.000000" false true))
      (:then_4))))

(event EventBeginPlay
  (bind _asgm_ld57 (Utilities|Casting|CastToGM_LD57 (Game|GetGameMode)))
  (Variables|Default|SetAs%20GM%20LD57 _asgm_ld57))

(event Collision|EventActorBeginOverlap
  (params (OtherActor :type Actor%20Object%20Reference)))

(event EventTick
  (params (DeltaSeconds :type Float%20%28single-precision%29)))

(fn ConstructionScript)