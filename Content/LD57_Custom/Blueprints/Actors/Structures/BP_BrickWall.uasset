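; BP_BrickWall is a destructible brick wall structure that pulses with the game's tempo and breaks when struck by a wrecking ball.
; It caches GM_LD57 on BeginPlay, then each Tick uses its Tempo value to lerp the wall's scale slightly around normal size.
; A Box hit by an actor tagged "wrecking-ball" triggers a camera shake, spawns the brick-burst Niagara effect and destroys the wall.
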(event OnComponentHit(BrickWall)
  (params (HitComponent :type Primitive%20Component%20Object%20Reference) (OtherActor :type Actor%20Object%20Reference) (OtherComp :type Primitive%20Component%20Object%20Reference) (NormalImpulse :type Vector :default "0, 0, 0") (Hit :type Hit%20Result%20Structure%20%28by%20ref%29)))

(event OnComponentHit(Box)
  (params (HitComponent :type Primitive%20Component%20Object%20Reference) (OtherActor :type Actor%20Object%20Reference) (OtherComp :type Primitive%20Component%20Object%20Reference) (NormalImpulse :type Vector :default "0, 0, 0") (Hit :type Hit%20Result%20Structure%20%28by%20ref%29))
  (if (Actor|ActorHasTag OtherActor "wrecking-ball")
    (Utilities|FlowControl|Sequence
      (:then_0
        (Game|Feedback|ClientStartCameraShake (Game|GetPlayerController 0) "/Game/LD57_Custom/Effects/BP_CameraShake.BP_CameraShake_C" 1.0 "World" "0, 0, 0"))
      (:then_1
        (Niagara|SpawnSystematLocation "/Game/LD57_Custom/Effects/NS_BrickBurst.NS_BrickBurst" (Transformation|GetActorLocation)))
      (:then_2
        (Actor|DestroyActor)))))

(event EventBeginPlay
  (bind _asgm_ld57 (Utilities|Casting|CastToGM_LD57 (Game|GetGameMode)))
  (Variables|Default|SetAs%20GM%20LD57 _asgm_ld57))

(event Collision|EventActorBeginOverlap
  (params (OtherActor :type Actor%20Object%20Reference)))

(event EventTick
  (params (DeltaSeconds :type Float%20%28single-precision%29))
  (bind _as_gm_ld57 (Variables|Default|GetAs%20GM%20LD57))
  (bind _tempo (Variables|/Game/LD57_Custom/Blueprints/Logic/GM_LD57.GM_LD57_C|GetTempo _as_gm_ld57))
  (bind _returnvalue (Math|Float|Lerp 0.95 1.05 _tempo))
  (Transformation|SetRelativeScale3D (Variables|Default|GetBrickWall) (Math|Vector|MakeVector _returnvalue _returnvalue _returnvalue)))

(fn ConstructionScript)