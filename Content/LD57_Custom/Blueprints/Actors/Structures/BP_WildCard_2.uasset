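; Wildcard barrel pickup that triggers a set or randomized effect once when the wrecking ball overlaps its capsule, then destroys itself after a delay.
; Effects explode, grow or shrink the paddle, or boost ball thrust.
; Chaos field strain breaks the Geometry Collection barrel; explosions add radial velocity, flip the ball's thrust direction and apply an impulse.
; Each effect plays a sound and sends alert text through GM_LD57.
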(event OnComponentHit(GC_Barrel)
  (params (HitComponent :type Primitive%20Component%20Object%20Reference) (OtherActor :type Actor%20Object%20Reference) (OtherComp :type Primitive%20Component%20Object%20Reference) (NormalImpulse :type Vector :default "0, 0, 0") (Hit :type Hit%20Result%20Structure%20%28by%20ref%29)))

(event OnComponentBeginOverlap(Capsule)
  (params (OverlappedComponent :type Primitive%20Component%20Object%20Reference) (OtherActor :type Actor%20Object%20Reference) (OtherComp :type Primitive%20Component%20Object%20Reference) (OtherBodyIndex :type Integer) (bFromSweep :type Boolean) (SweepResult :type Hit%20Result%20Structure%20%28by%20ref%29))
  (if (Actor|ActorHasTag OtherActor "wrecking-ball")
    (Utilities|FlowControl|DoOnce false
      (:Completed
        (CallFunction|HandleWildCardEffect)
        (Utilities|FlowControl|Delay 5.0)
        (Actor|DestroyActor)))))

(event EventBeginPlay
  (if (Variables|Default|GetRandomizeType)
    (bind _output_get (Variables|Default|SetWildCardType (.OutItem (Utilities|Array|Random (Utilities|Array|MakeArray "NewEnumerator0" "NewEnumerator1" "NewEnumerator2" "NewEnumerator3")))))
    (Development|PrintString (Utilities|String|EnumtoString _output_get))))

(event Collision|EventActorBeginOverlap
  (params (OtherActor :type Actor%20Object%20Reference)))

(event EventTick
  (params (DeltaSeconds :type Float%20%28single-precision%29)))

(fn ConstructionScript)

(fn HandleWildCardEffect
  (switch Utilities|FlowControl|Switch|SwitchonENUM_WildCardTypes (Variables|Default|GetWildCardType)
    (:NewEnumerator0
      (CallFunction|Explode))
    (:NewEnumerator1
      (CallFunction|GrowPaddle))
    (:NewEnumerator2
      (CallFunction|ShrinkPaddle))
    (:NewEnumerator3
      (CallFunction|SpeedUp))))

(fn Explode
  (bind _radialfalloff (Variables|Default|GetRadialFalloff))
  (bind _fieldtarget (Variables|Default|GetFieldTarget))
  (bind _returnvalue (Transformation|GetWorldLocation _fieldtarget))
  (bind _sphereradius (Variables|/Script/Engine.SphereComponent|GetSphereRadius _fieldtarget))
  (bind _returnvalue_2 (Field|SetRadialFalloff _radialfalloff 5e+05 0.0 1.0 0.0 _sphereradius _returnvalue "Field_FallOff_None"))
  (Class|FieldSystemComponent|ApplyPhysicsField (Variables|Default|GetFieldSystem) true "Field_ExternalClusterStrain" 0 _returnvalue_2)
  (Class|FieldSystemComponent|ApplyPhysicsField (Variables|Default|GetFieldSystem) true "Field_LinearVelocity" 0 (Field|SetCullingField (Variables|Default|GetCullingField) _returnvalue_2 (Field|SetRadialVector (Variables|Default|GetRadialVector) 1e+03 _returnvalue) "Field_Culling_Outside"))
  (Niagara|SpawnSystematLocation "/Game/LD57_Custom/Effects/NS_Explosion.NS_Explosion" (Transformation|GetWorldLocation (Variables|Default|GetGC_Barrel)))
  (bind _returnvalue_3 (Actor|GetActorOfClass "/Game/LD57_Custom/Blueprints/Actors/BP_WreckingBall.BP_WreckingBall_C"))
  (Variables|/Game/LD57_Custom/Blueprints/Actors/BP_WreckingBall.BP_WreckingBall_C|SetThrustDirection _returnvalue_3 (* (Variables|/Game/LD57_Custom/Blueprints/Actors/BP_WreckingBall.BP_WreckingBall_C|GetThrustDirection _returnvalue_3) -1.0))
  (Physics|AddImpulse (Variables|/Game/LD57_Custom/Blueprints/Actors/BP_WreckingBall.BP_WreckingBall_C|GetSphere _returnvalue_3) (* (* (Variables|/Game/LD57_Custom/Blueprints/Actors/BP_WreckingBall.BP_WreckingBall_C|GetThrustDirection _returnvalue_3) -1.0) 2e+05) "None" false)
  (Audio|PlaySound2D "/Game/LD57_Custom/Audio/FX/Explosion23_Cue.Explosion23_Cue" 1.0 1.0 0.0 0 0)
  (CallFunction|AlertEffect "Boom"))

(fn GrowPaddle
  (CallFunction|BreakBarrel)
  (bind _returnvalue (Actor|GetActorOfClass "/Game/LD57_Custom/Blueprints/Actors/BP_PaddlePawn.BP_PaddlePawn_C"))
  (Transformation|SetRelativeScale3D (Variables|/Game/LD57_Custom/Blueprints/Actors/BP_PaddlePawn.BP_PaddlePawn_C|GetPaddle _returnvalue) (* (Variables|/Script/Engine.SceneComponent|GetRelativeScale3D (Variables|/Game/LD57_Custom/Blueprints/Actors/BP_PaddlePawn.BP_PaddlePawn_C|GetPaddle _returnvalue)) 1.25))
  (Audio|PlaySound2D "/Game/LD57_Custom/Audio/FX/GrowNoise_Cue.GrowNoise_Cue" 1.0 1.0 0.0 0 0)
  (CallFunction|AlertEffect "Paddle Size Up"))

(fn ShrinkPaddle
  (CallFunction|BreakBarrel)
  (bind _returnvalue (Actor|GetActorOfClass "/Game/LD57_Custom/Blueprints/Actors/BP_PaddlePawn.BP_PaddlePawn_C"))
  (Transformation|SetRelativeScale3D (Variables|/Game/LD57_Custom/Blueprints/Actors/BP_PaddlePawn.BP_PaddlePawn_C|GetPaddle _returnvalue) (* (Variables|/Script/Engine.SceneComponent|GetRelativeScale3D (Variables|/Game/LD57_Custom/Blueprints/Actors/BP_PaddlePawn.BP_PaddlePawn_C|GetPaddle _returnvalue)) 0.8))
  (Audio|PlaySound2D "/Game/LD57_Custom/Audio/FX/ShrinkNoise_Cue.ShrinkNoise_Cue" 1.0 1.0 0.0 0 0)
  (CallFunction|AlertEffect "Paddle Size Down"))

(fn SpeedUp
  (CallFunction|BreakBarrel)
  (bind _returnvalue (Actor|GetActorOfClass "/Game/LD57_Custom/Blueprints/Actors/BP_WreckingBall.BP_WreckingBall_C"))
  (Variables|/Script/Engine.PhysicsThrusterComponent|SetThrustStrength (Variables|/Game/LD57_Custom/Blueprints/Actors/BP_WreckingBall.BP_WreckingBall_C|GetPhysicsThruster _returnvalue) (* (Variables|/Script/Engine.PhysicsThrusterComponent|GetThrustStrength (Variables|/Game/LD57_Custom/Blueprints/Actors/BP_WreckingBall.BP_WreckingBall_C|GetPhysicsThruster _returnvalue)) 1.5))
  (Audio|PlaySound2D "/Game/LD57_Custom/Audio/FX/GrowNoise_Cue.GrowNoise_Cue" 1.0 1.0 0.0 0 0)
  (CallFunction|AlertEffect "Speed Up"))

(fn AlertEffect
  (params (AlertText :type String))
  (bind _asgm_ld57 (Utilities|Casting|CastToGM_LD57 (Game|GetGameMode)))
  (Default|CallAlertDispatcher _asgm_ld57 AlertText))

(fn BreakBarrel
  (bind _fieldtarget (Variables|Default|GetFieldTarget))
  (Class|FieldSystemComponent|ApplyPhysicsField (Variables|Default|GetFieldSystem) true "Field_ExternalClusterStrain" 0 (Field|SetRadialFalloff (Variables|Default|GetRadialFalloff) 5e+05 0.0 1.0 0.0 (Variables|/Script/Engine.SphereComponent|GetSphereRadius _fieldtarget) (Transformation|GetWorldLocation _fieldtarget) "Field_FallOff_None")))