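; BP_WreckingBall is a physics-driven ball that steers its thrust by bouncing off tagged surfaces.
; Its thrust direction starts opposite the actor's forward vector, and Tick turns the PhysicsThruster's world rotation to match it each frame.
; When Sphere hits an actor tagged "bounce-ball", the direction reflects off the hit normal and is flattened to the horizontal plane.
; Sphere1 hits only print a debug message.
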(event OnComponentHit(Sphere)
  (params (HitComponent :type Primitive%20Component%20Object%20Reference) (OtherActor :type Actor%20Object%20Reference) (OtherComp :type Primitive%20Component%20Object%20Reference) (NormalImpulse :type Vector :default "0, 0, 0") (Hit :type Hit%20Result%20Structure%20%28by%20ref%29))
  (if (Actor|ActorHasTag OtherActor "bounce-ball")
    (Variables|Default|SetThrustDirection (* (Math|Vector|GetReflectionVector (Variables|Default|GetThrustDirection) (.Normal (Collision|BreakHitResult Hit))) "1.000000,1.000000,0.000000"))))

(event OnComponentBeginOverlap(Sphere)
  (params (OverlappedComponent :type Primitive%20Component%20Object%20Reference) (OtherActor :type Actor%20Object%20Reference) (OtherComp :type Primitive%20Component%20Object%20Reference) (OtherBodyIndex :type Integer) (bFromSweep :type Boolean) (SweepResult :type Hit%20Result%20Structure%20%28by%20ref%29)))

(event OnComponentHit(Sphere1)
  (params (HitComponent :type Primitive%20Component%20Object%20Reference) (OtherActor :type Actor%20Object%20Reference) (OtherComp :type Primitive%20Component%20Object%20Reference) (NormalImpulse :type Vector :default "0, 0, 0") (Hit :type Hit%20Result%20Structure%20%28by%20ref%29))
  (Development|PrintString "Hit"))

(event EventBeginPlay
  (Variables|Default|SetThrustDirection (* (Transformation|GetActorForwardVector) -1.0)))

(event Collision|EventActorBeginOverlap
  (params (OtherActor :type Actor%20Object%20Reference)))

(event EventTick
  (params (DeltaSeconds :type Float%20%28single-precision%29))
  (Transformation|SetWorldRotation (Variables|Default|GetPhysicsThruster) (Math|Conversions|RotationFromXVector (Variables|Default|GetThrustDirection)) false false))

(fn ConstructionScript)